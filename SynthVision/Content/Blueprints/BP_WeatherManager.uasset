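; Weather manager that drives sun angle, fog, rain, snow and wind, applying its configured values at BeginPlay.
; Setter events rotate the tagged sun, set tagged height fog density, and feed Niagara systems and MPC_WeatherState wetness and wind parameters.
; Rain and snow are mutually exclusive: each zeroes the other's particles and overwrites shared wetness and fog.
; Snow is applied after rain at startup, so its values win.
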(event Custom|SetTimeOfDay
  (params (NewTime :type Float%20%28double-precision%29))
  (bind _outactors (Actor|GetAllActorswithTag "SunLight"))
  (Transformation|SetActorRotation (Utilities|Array|Get(acopy) _outactors) (Math|Rotator|MakeRotator 0.0 (- 9e+01 (* NewTime 15.0)) 0.0)))

(event Custom|SetFogDensity
  (params (NewFog :type Float%20%28double-precision%29))
  (bind _outactors (Actor|GetAllActorswithTag "Fog"))
  (bind _asexponential_height_fog (Utilities|Casting|CastToExponentialHeightFog (Utilities|Array|Get(acopy) _outactors)))
  (Class|ExponentialHeightFogComponent|SetFogDensity (Variables|/Script/Engine.ExponentialHeightFog|GetComponent _asexponential_height_fog) (* NewFog (Variables|Default|GetMaxFogDensity))))

(event Custom|SetRainIntensity
  (params (NewRainIntensity :type Float%20%28double-precision%29))
  (Rendering|Material|SetScalarParameterValue "/Game/Materials/MPC/MPC_WeatherState.MPC_WeatherState" "WetnessAmount" NewRainIntensity :!class /Script/Engine.KismetMaterialLibrary)
  (CallFunction|SetFogDensity (* NewRainIntensity (Variables|Default|GetMaxFog)))
  (Niagara|SetNiagaraVariable(Float) (Variables|Default|GetRain) "RainIntensity" NewRainIntensity)
  (Niagara|SetNiagaraVariable(Float) (Variables|Default|GetSnow) "SnowIntensity" 0.0))

(event Custom|SetSnowIntensity
  (params (NewSnowIntensity :type Float%20%28double-precision%29))
  (Rendering|Material|SetScalarParameterValue "/Game/Materials/MPC/MPC_WeatherState.MPC_WeatherState" "WetnessAmount" NewSnowIntensity :!class /Script/Engine.KismetMaterialLibrary)
  (CallFunction|SetFogDensity (* NewSnowIntensity (Variables|Default|GetMaxFog)))
  (Niagara|SetNiagaraVariable(Float) (Variables|Default|GetSnow) "SnowIntensity" NewSnowIntensity)
  (Niagara|SetNiagaraVariable(Float) (Variables|Default|GetRain) "RainIntensity" 0.0))

(event Custom|SetWindSpeed
  (params (NewWindStrength :type Float%20%28double-precision%29))
  (bind _windmaxstrength (Variables|Default|GetWindMaxStrength))
  (bind _returnvalue (* NewWindStrength _windmaxstrength))
  (Rendering|Material|SetScalarParameterValue "/Game/Materials/MPC/MPC_WeatherState.MPC_WeatherState" "WindStrength" NewWindStrength :!class /Script/Engine.KismetMaterialLibrary)
  (Class|NiagaraComponent|SetNiagaraVariableVec3 (Variables|Default|GetSnow) "WindDirection" _returnvalue)
  (Class|NiagaraComponent|SetNiagaraVariableVec3 (Variables|Default|GetRain) "WindDirection" _returnvalue))

(event EventBeginPlay
  (CallFunction|SetTimeOfDay (Variables|Default|GetTimeOfDay))
  (CallFunction|SetFogDensity (Variables|Default|GetFogDensity))
  (CallFunction|SetRainIntensity (Variables|Default|GetRainIntensity))
  (CallFunction|SetSnowIntensity (Variables|Default|GetSnowIntensity))
  (CallFunction|SetWindSpeed (Variables|Default|GetWindStrength)))

(fn ConstructionScript)