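; BP_Tree is a procedural tree actor assembled in its construction script from a seed, with no runtime logic.
; The seed picks trunk and branch meshes, both indexed by the trunk array's length, and varies trunk scale and yaw.
; Each branch socket gets a canopy mesh varied by a re-seeded stream.
; Cleanup searches for "Canopy" component tags, but new canopies only trigger a gameplay tag container addition.
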(event EventBeginPlay)

(event Collision|EventActorBeginOverlap
  (params (OtherActor :type Actor%20Object%20Reference)))

(event EventTick
  (params (DeltaSeconds :type Float%20%28single-precision%29)))

(fn ConstructionScript
  (bind _trunkmeshes (Variables|Default|GetTrunkMeshes))
  (bind _seed (Variables|Default|GetSeed))
  (bind _trunk (Variables|Default|GetTrunk))
  (bind _seed_2 (Variables|Default|GetSeed))
  (bind _returnvalue (Utilities|Array|Length _trunkmeshes))
  (bind _returnvalue_2 (Math|Random|MakeRandomStream _seed_2))
  (bind _returnvalue_3 (Math|Random|MakeRandomStream _seed))
  (bind _returnvalue_4 (Math|Random|RandomFloatinRangefromStream _returnvalue_3 0.9 1.2))
  (bind _returnvalue_5 (- _returnvalue 1))
  (bind _returnvalue_6 (Class|KismetMathLibrary|RandomIntegerfromStream _returnvalue_2 _returnvalue_5))
  (for _array_element (Actor|GetComponentsbyTag "/Script/Engine.StaticMeshComponent" "Canopy")
    (Components|DestroyComponent _array_element))
  (Components|StaticMesh|SetStaticMesh (Variables|Default|GetTrunk) (Utilities|Array|Get(acopy) (Variables|Default|GetTrunkMeshes) _returnvalue_6))
  (Components|StaticMesh|SetStaticMesh (Variables|Default|GetBranches) (Utilities|Array|Get(acopy) (Variables|Default|GetBranchMeshes) _returnvalue_6))
  (Transformation|SetRelativeScale3D _trunk (Math|Vector|MakeVector _returnvalue_4 _returnvalue_4 _returnvalue_4))
  (Transformation|SetRelativeRotation _trunk (Math|Rotator|MakeRotator 0.0 0.0 (Math|Random|RandomFloatinRangefromStream _returnvalue_3 0.0 3.6e+02)) false false)
  (LocalVariables|SetLocalStream (Math|Random|MakeRandomStream (Variables|Default|GetSeed)))
  (for _array_element_2 (Transformation|GetAllSocketNames (Variables|Default|GetBranches))
    (LocalVariables|SetLocalStream (Math|Random|MakeRandomStream (Class|KismetMathLibrary|RandomIntegerfromStream (LocalVariables|GetLocalStream) 10)))
    (bind _returnvalue_7 (AddComponent|AddStaticMeshComponent false))
    (GameplayTags|AddGameplayTag (Variables|Default|GetTagContainer) "(TagName=\"Canopy\")" :!class /Script/GameplayTags.BlueprintGameplayTagLibrary)
    (Components|StaticMesh|SetStaticMesh _returnvalue_7 (Utilities|Array|Get(acopy) (Variables|Default|GetCanopyMeshes) (Class|KismetMathLibrary|RandomIntegerfromStream (LocalVariables|GetLocalStream) (- (Utilities|Array|Length (Variables|Default|GetCanopyMeshes)) 1))))
    (Transformation|AttachComponentToComponent _returnvalue_7 (Variables|Default|GetBranches) _array_element_2 "SnapToTarget" "SnapToTarget" "KeepRelative" true)
    (Transformation|SetRelativeScale3D _returnvalue_7 (Math|Vector|MakeVector (Math|Random|RandomFloatinRangefromStream (LocalVariables|GetLocalStream) 0.005 0.007) (Math|Random|RandomFloatinRangefromStream (LocalVariables|GetLocalStream) 0.005 0.007) (Math|Random|RandomFloatinRangefromStream (LocalVariables|GetLocalStream) 0.005 0.007)))
    (Transformation|SetRelativeRotation _returnvalue_7 (Math|Rotator|MakeRotator 0.0 0.0 (Math|Random|RandomFloatinRangefromStream (LocalVariables|GetLocalStream) 0.0 3.6e+02)) false false)))